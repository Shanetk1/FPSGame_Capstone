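; First-person player character that spawns a BP_WeaponMaster on BeginPlay, attaches it to the mesh's Grip_Point socket and drives it from input.
; Fire and fire-mode inputs are forwarded to the weapon, while Aim toggles IsAiming.
; Each tick points the weapon's muzzle rotation at AimObject and interpolates FPPCam to the weapon's camera when aiming, or back to the head socket otherwise.
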(event `self.ReceiveBeginPlay`
  (bind _returnvalue (`|SpawnActorFromClass` "/Game/Weapons/BP_WeaponMaster.BP_WeaponMaster_C" (`KismetMathLibrary.MakeTransform` (0.0 0.0 0.0)) "AlwaysSpawn" "OverrideRootScale" null null))
  (bind _output_get (set `self.EquippedWeapon` _returnvalue))
  (`self.K2_AttachToComponent` _output_get (`self.Mesh`) "Grip_Point" "KeepRelative" "KeepRelative" "KeepRelative" true))

(event `InputAction|Fire`
  (params (Key :type "Key Structure"))
  (bind _equippedweapon (`self.EquippedWeapon`))
  ;[1 1 1] Fire Input
  (:`Pressed`
    (`self.setWeaponRotation`)
    (`/Game/Weapons/BP_WeaponMaster.StartFire` _equippedweapon))
  (:`Released`
    (`/Game/Weapons/BP_WeaponMaster.StopFire` _equippedweapon)))

(event `self.ReceiveTick`
  (params (DeltaSeconds :type "Float (single-precision)"))
  ;[1 1 1] Tick
  (`|ExecutionSequence`
    (:`then_0`
      (`self.setWeaponRotation`))
    (:`then_1`
      (if (`self.isAiming`)
        (`self.AimDownSight`)
        (else
          (`self.UnAim`))))))

(event `InputAction|FireMode`
  (params (Key :type "Key Structure"))
  (:`Pressed`
    (`/Game/Weapons/BP_WeaponMaster.FireModeSwitch` (`self.EquippedWeapon`))))

(event `InputAction|Aim`
  (params (Key :type "Key Structure"))
  (bind _equippedweapon (`self.EquippedWeapon`))
  (:`Pressed`
    (`/Engine/EditorBlueprintResources/StandardMacros.IsValid` _equippedweapon
      (:`Is Valid`
        (set `self.isAiming` true))))
  (:`Released`
    (`/Engine/EditorBlueprintResources/StandardMacros.IsValid` _equippedweapon
      (:`Is Valid`
        (set `self.isAiming` false)))))

(fn `AimDownSight`
  (locals (NewLocalVar_0 :type "Rotator Structure" :default (struct)))
  (bind _returnvalue (`GameplayStatics.GetWorldDeltaSeconds`))
  (bind _fppcam (`self.FPPCam`))
  (bind _camera (`/Game/Weapons/BP_WeaponMaster.Camera` (`self.EquippedWeapon`)))
  (`ActorComponent.Deactivate` (`self.ADSCamera`))
  (`ActorComponent.Activate` _fppcam false)
  (`SceneComponent.K2_SetWorldLocationAndRotation` _fppcam (`KismetMathLibrary.VInterpTo` (`SceneComponent.K2_GetComponentLocation` _fppcam) (`SceneComponent.K2_GetComponentLocation` _camera) _returnvalue 15.0) (`KismetMathLibrary.RInterpTo` (`SceneComponent.K2_GetComponentRotation` _fppcam) (`SceneComponent.K2_GetComponentRotation` _camera) _returnvalue 15.0) false false))

(fn `setWeaponRotation`
  (bind _equippedweapon (`self.EquippedWeapon`))
  (set `/Game/Weapons/BP_WeaponMaster.MuzzleRotation` (`KismetMathLibrary.FindLookAtRotation` (`SceneComponent.GetSocketLocation` (`/Game/Objects/BP_ObjectMaster.SkeletalMesh` _equippedweapon) "Muzzle") (`SceneComponent.K2_GetComponentLocation` (`self.AimObject`))) _equippedweapon))

(fn `UnAim`
  (bind _returnvalue (`GameplayStatics.GetWorldDeltaSeconds`))
  (bind _mesh (`self.Mesh`))
  (bind _fppcam (`self.FPPCam`))
  (bind _fppcam_2 (`self.FPPCam`))
  (bind _returnvalue_location (`KismetMathLibrary.BreakTransform` (`SceneComponent.K2_GetComponentToWorld` _fppcam_2)))
  (bind _returnvalue_2 (`SceneComponent.K2_GetComponentLocation` _fppcam))
  (`SceneComponent.K2_SetWorldLocationAndRotation` (`self.FPPCam`) (`KismetMathLibrary.VInterpTo` _returnvalue_2 (`SceneComponent.GetSocketLocation` _mesh "head") _returnvalue 15.0) (`KismetMathLibrary.RInterpTo` (`SceneComponent.K2_GetComponentRotation` _fppcam) (`SceneComponent.GetSocketRotation` _mesh "head") _returnvalue 15.0) false false)
  (if (== _returnvalue_2 _returnvalue_location :`ErrorTolerance` 0.01)
    (`ActorComponent.Deactivate` _fppcam)
    (`ActorComponent.Activate` _fppcam_2 false)))

(fn `UserConstructionScript`)